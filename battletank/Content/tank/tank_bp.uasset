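; Player-controlled tank pawn Blueprint that wires input to aiming, movement and camera control.
; On BeginPlay it initializes the TankAiming and TankMovement components with its barrel, turret and tracks, and passes itself to the healthbar widget.
; Axis input rotates the azimuth gimbal and spring arm with frame-time scaling and sends drive intent to TankMovement.
; Actions fire through TankAiming, toggle first- and third-person cameras, or quit the game.
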(event `self.ReceiveBeginPlay`
  (`TankAimingComponent.initialize` (`self.TankAiming`) (`self.Barrel`) (`self.Turret`))
  (`TankMovementComponent.initialize` (`self.TankMovement`) (`self.lefttrack`) (`self.righttrack`))
  (`self.healthbarfunc`))

(event `InputAxis|aimazimuthal`
  (params (AxisValue :type "Float (single-precision)"))
  ;[1 1 1] input bindings
  (`SceneComponent.K2_AddLocalRotation` (`self.azimuthal gimbal`) (`KismetMathLibrary.MakeRotator` 0.0 0.0 (* (`GameplayStatics.GetWorldDeltaSeconds`) AxisValue 100.0)) false false))

(event `InputAxis|aimaltitude`
  (params (AxisValue :type "Float (single-precision)"))
  ;[1 1 1] input bindings
  (`SceneComponent.K2_AddLocalRotation` (`self.SpringArm`) (`KismetMathLibrary.MakeRotator` 0.0 (* AxisValue (`GameplayStatics.GetWorldDeltaSeconds`) 100.0)) false false))

(event `InputAxis|move forward`
  (params (AxisValue :type "Float (single-precision)"))
  ;[1 1 1] movement
  (`TankMovementComponent.intendtomoveforward` (`self.TankMovement`) AxisValue))

(event `InputAxis|moverotation`
  (params (AxisValue :type "Float (single-precision)"))
  ;[1 1 1] movement
  (`TankMovementComponent.intendtorotated` (`self.TankMovement`) AxisValue))

(event `InputAction|fire`
  (params (Key :type "Key Structure"))
  ;[1 1 1] input bindings
  (:`Pressed`
    (`TankAimingComponent.fire` (`self.TankAiming`))))

(event `InputAction|SWITCH CAMERAS`
  (params (Key :type "Key Structure"))
  ;[1 1 1] input bindings
  (:`Pressed`
    (`self.switch cameras`)))

(event `InputAction|quit`
  (params (Key :type "Key Structure"))
  ;[1 1 1] input bindings
  (:`Pressed`
    (`KismetSystemLibrary.QuitGame` null "Quit")))

(fn `healthbarfunc`
  (bind _ashealthbar (cast `/Game/userinterface/healthbar` (`WidgetComponent.GetUserWidgetObject` (`self.Widget`)))
    (:`then`
      (set `/Game/userinterface/healthbar.tank` self _ashealthbar))
    (:`CastFailed`
      _))
  (return))

(fn `switch cameras`
  (`ActorComponent.ToggleActive` (`self.1ST PERSON`))
  (`ActorComponent.ToggleActive` (`self.3RD PERSON`))
  (return))

(fn `UserConstructionScript`)